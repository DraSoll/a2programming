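; BP_Button is a toggle button that spawns a BP_MovingUp platform and reveals three keys hidden at BeginPlay.
; Each ButtonPressed call spawns the platform at the Spawn location, destroying the previous one after the first press, and toggles Pressed to swap the button material.
; The FirstTime flag limits the key reveal to the initial press.
; Every press flashes a short-lived sparks effect; the Use function is empty.
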(event Custom|ButtonPressed
  (if (Variables|Default|GetFirstTime) ; This checks if the button has been pressed already
    _
    (else
      (Actor|DestroyActor (stale _returnvalue)) ; Destroys the platform if it exists already
    ))
  ;[1 1 1] First time spawns the platform
  (bind _returnvalue (Game|SpawnActorfromClass "/Game/Blueprints/BP_MovingUp.BP_MovingUp_C" (Math|Conversions|ToTransform(Vector) (Transformation|GetActorLocation (Variables|Default|GetSpawn))) "Undefined" "MultiplyWithRoot" 0 0))
  (if (Variables|Default|GetPressed?)
    (Variables|Default|SetPressed? false)
    (Rendering|Material|SetMaterial (Variables|Default|GetButton) 0 "/Engine/EngineDebugMaterials/HeatmapMaterial.HeatmapMaterial")
    (else
      (Variables|Default|SetPressed? true)
      ;[1 1 1] This is to do with the visibility of the keys in the level
      (if (!= (Variables|Default|GetFirstTime) true)
        _
        (else
          ;[1 1 1] Show hidden keys to the player
          (Rendering|SetActorHiddenInGame (Variables|Default|GetKey3) false)
          (Rendering|SetActorHiddenInGame (Variables|Default|GetKey2) false)
          (Rendering|SetActorHiddenInGame (Variables|Default|GetKey1) false)
          (Variables|Default|SetFirstTime false)))
      (Rendering|Material|SetMaterial (Variables|Default|GetButton) 0 "/Engine/MapTemplates/Materials/BasicAsset03.BasicAsset03") ; Changes the button to greem
    ))
  ;[1 1 1] Spawn Sparks
  (bind _returnvalue_2 (Game|SpawnActorfromClass "/Game/StarterContent/Blueprints/Blueprint_Effect_Sparks.Blueprint_Effect_Sparks_C" (Math|Conversions|ToTransform(Vector) (Transformation|GetActorLocation (Variables|Default|GetParticle))) "Undefined" "MultiplyWithRoot" 0 0))
  (Utilities|FlowControl|Delay 0.2)
  (Actor|DestroyActor _returnvalue_2))

(event EventBeginPlay
  ;[1 1 1] Hide Keys
  (Rendering|SetActorHiddenInGame (Variables|Default|GetKey3) true)
  (Rendering|SetActorHiddenInGame (Variables|Default|GetKey2) true)
  (Rendering|SetActorHiddenInGame (Variables|Default|GetKey1) true)
  (Variables|Default|SetFirstTime true))

(fn ConstructionScript)

(fn Use)