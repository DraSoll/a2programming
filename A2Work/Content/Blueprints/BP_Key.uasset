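; BP_Key is a collectible key pickup that adds to the player's key count.
; When its component R is overlapped, it casts player pawn 0 to BP_ThirdPersonCharacter without checking the overlapping actor, then increments KeyCollected.
; It prints the new count, plays a ding sound, spawns a collect effect, calls the character's CallKeyUpdated and destroys itself.
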(event OnComponentBeginOverlap(R)
  (params (OverlappedComponent :type Primitive%20Component%20Object%20Reference) (OtherActor :type Actor%20Object%20Reference) (OtherComp :type Primitive%20Component%20Object%20Reference) (OtherBodyIndex :type Integer) (bFromSweep :type Boolean) (SweepResult :type Hit%20Result%20Structure%20%28by%20ref%29))
  (bind _asbp_third_person_character (Utilities|Casting|CastToBP_ThirdPersonCharacter (Game|Player|GetPlayerPawn 0)))
  (bind _output_get (Variables|/Game/ThirdPerson/Blueprints/BP_ThirdPersonCharacter.BP_ThirdPersonCharacter_C|SetKeyCollected _asbp_third_person_character (+ 1 (Variables|/Game/ThirdPerson/Blueprints/BP_ThirdPersonCharacter.BP_ThirdPersonCharacter_C|GetKeyCollected _asbp_third_person_character))))
  (Development|PrintString (Utilities|String|ToString(Integer) _output_get))
  (Audio|PlaySound2D "/Game/imported/DingCue.DingCue" 1.0 1.0 0.0 0 0)
  (Niagara|SpawnSystematLocation "/Game/imported/FX_KeyCollect.FX_KeyCollect" (Transformation|GetActorLocation))
  (Default|CallKeyUpdated _asbp_third_person_character)
  (Actor|DestroyActor))

(event EventBeginPlay)

(event Collision|EventActorBeginOverlap
  (params (OtherActor :type Actor%20Object%20Reference)))

(event EventTick
  (params (DeltaSeconds :type Float%20%28single-precision%29)))

(fn ConstructionScript)