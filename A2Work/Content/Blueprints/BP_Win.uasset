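; BP_Win is a level-completion trigger that celebrates a win and returns the game to the MainMenu level.
; Any overlap with its Box plays a win sound and loops to spawn NS_WIn Niagara effects at random points within the bounds of TriggerBox1 and TriggerBox2.
; The Delay sits inside the loop body, so the effects spawn at once and MainMenu opens after a single five-second wait.
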(event OnComponentBeginOverlap(Box)
  (params (OverlappedComponent :type Primitive%20Component%20Object%20Reference) (OtherActor :type Actor%20Object%20Reference) (OtherComp :type Primitive%20Component%20Object%20Reference) (OtherBodyIndex :type Integer) (bFromSweep :type Boolean) (SweepResult :type Hit%20Result%20Structure%20%28by%20ref%29))
  (bind _triggerbox1 (Variables|Default|GetTriggerBox1))
  (bind _triggerbox2 (Variables|Default|GetTriggerBox2))
  (bind (_origin _boxextent) (Collision|GetActorBounds _triggerbox2 false false))
  (bind (_origin_2 _boxextent_2) (Collision|GetActorBounds _triggerbox1 false false))
  (Audio|PlaySoundatLocation "/Game/imported/make_more_sound-8-bit-video-game-win-level-sound-version-1-145827_1_.make_more_sound-8-bit-video-game-win-level-sound-version-1-145827_1_" (Transformation|GetActorLocation) "0, 0, 0" 1.0 1.0 0.0 0 0 0 0)
  (for _index (range 0 10)
    (Niagara|SpawnSystematLocation "/Game/imported/NS_WIn.NS_WIn" (Math|Random|RandomPointinBoundingBox _origin_2 _boxextent_2) "0, 0, 0" "1.000000,1.000000,1.000000" false)
    (Niagara|SpawnSystematLocation "/Game/imported/NS_WIn.NS_WIn" (Math|Random|RandomPointinBoundingBox _origin _boxextent) "0, 0, 0" "1.000000,1.000000,1.000000" false)
    (Utilities|FlowControl|Delay 5.0)
    (Game|OpenLevel(byName) "MainMenu")))

(event EventBeginPlay)

(event Collision|EventActorBeginOverlap
  (params (OtherActor :type Actor%20Object%20Reference)))

(event EventTick
  (params (DeltaSeconds :type Float%20%28single-precision%29)))

(fn ConstructionScript)