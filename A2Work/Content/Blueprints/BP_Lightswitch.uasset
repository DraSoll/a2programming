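; BP_Lightswitch controls three spotlights that show the player's key collection progress by turning red one at a time.
; BeginPlay resets each light to a dim grey.
; The KeyCollected event reads the key count from BP_ThirdPersonCharacter and reddens the spotlight matching a count of one, two or three.
; Each spotlight is referenced individually; SpotlightArray is unused.
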(event Custom|KeyCollected
  (bind _returnvalue (Math|Color|SelectColor "(R=1.000000,G=0.000000,B=0.010357,A=1.000000)" "(R=1.000000,G=0.000000,B=0.024945,A=1.000000)" false))
  (bind _asbp_third_person_character (Utilities|Casting|CastToBP_ThirdPersonCharacter (Game|GetPlayerCharacter 0)))
  ;[1 1 1] Turn light red w/first key
  (if (== (Variables|/Game/ThirdPerson/Blueprints/BP_ThirdPersonCharacter.BP_ThirdPersonCharacter_C|GetKeyCollected _asbp_third_person_character) 1)
    (Rendering|Components|Light|SetLightColor (Variables|/Script/Engine.Light|GetLightComponent (Variables|Default|GetRedSpotlight1)) _returnvalue true)
    (else
      ;[1 1 1] Turn light red w/2nd key
      (if (== (Variables|/Game/ThirdPerson/Blueprints/BP_ThirdPersonCharacter.BP_ThirdPersonCharacter_C|GetKeyCollected _asbp_third_person_character) 2)
        (Rendering|Components|Light|SetLightColor (Variables|/Script/Engine.Light|GetLightComponent (Variables|Default|GetRedSpotlight2)) _returnvalue true)
        (else
          ;[1 1 1] CommenTurnt
          (if (== (Variables|/Game/ThirdPerson/Blueprints/BP_ThirdPersonCharacter.BP_ThirdPersonCharacter_C|GetKeyCollected _asbp_third_person_character) 3)
            (Rendering|Components|Light|SetLightColor (Variables|/Script/Engine.Light|GetLightComponent (Variables|Default|GetRedSpotlight3)) _returnvalue true)))))))

(event EventBeginPlay
  ;[1 1 1] Reset lights
  (Rendering|Components|Light|SetLightColor (Variables|/Script/Engine.Light|GetLightComponent (Variables|Default|GetRedSpotlight1)) "(R=0.244792,G=0.244792,B=0.244792,A=1.000000)" true)
  (Rendering|Components|Light|SetLightColor (Variables|/Script/Engine.Light|GetLightComponent (Variables|Default|GetRedSpotlight3)) "(R=0.192708,G=0.192708,B=0.192708,A=1.000000)" true)
  (Rendering|Components|Light|SetLightColor (Variables|/Script/Engine.Light|GetLightComponent (Variables|Default|GetRedSpotlight2)) "(R=0.272570,G=0.272570,B=0.272570,A=1.000000)" true))

(fn ConstructionScript)